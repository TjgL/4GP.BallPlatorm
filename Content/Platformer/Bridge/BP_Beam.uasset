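; BP_Beam is a bridge beam actor that links a Start and an End connector actor.
; On each LiveLink controller update, it checks HasConnectors, then teleports to the connectors' midpoint and draws a debug line and point.
; GetForceAtConnector holds unfinished spring-damper force math that is disconnected, so it computes nothing.
; The validity check in HasConnectors is likewise left unwired.
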(event `self.LiveLinkComponentController.OnLiveLinkUpdated`
  (params (DeltaTime :type "Float (single-precision)"))
  (bind _returnvalue (`self.K2_GetActorLocation` (`self.End`)))
  (bind _returnvalue_2 (`self.K2_GetActorLocation` (`self.Start`)))
  (bind _returnvalue_3 (+ (/ (- _returnvalue _returnvalue_2) 2) _returnvalue_2))
  (if (`self.HasConnectors`)
    (`KismetSystemLibrary.DrawDebugLine` _returnvalue_2 _returnvalue (struct :`R` 0.271419 :`G` 1.0 :`A` 1.0) 0.1 1.0)
    (`KismetSystemLibrary.DrawDebugPoint` _returnvalue_3 10.0 (struct :`R` 1.0 :`A` 1.0))
    (`self.K2_SetActorLocation` _returnvalue_3 false true)))

(fn `GetForceAtConnector`
  (params (Connector :type "/Game/Platformer/Bridge/BP_Connector Object Reference"))
  (returns (Force :type "Vector Structure"))
  (locals (Length :type "Vector Structure") (VelocityDamping :type "Vector Structure") (ForceBeam :type "Vector Structure")))

(fn `UserConstructionScript`)