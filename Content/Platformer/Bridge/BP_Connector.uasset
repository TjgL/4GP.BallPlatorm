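; BP_Connector is a bridge joint sphere that links beams, acting either as a fixed anchor or a physics-driven node.
; Each tick, a non-anchor connector sums the force every attached beam reports for it and applies that total to its sphere.
; The construction script picks an anchor or connector material and enables physics simulation and gravity only for non-anchors.
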(event `self.ReceiveTick`
  (params (DeltaSeconds :type "Float (single-precision)"))
  (if (not (`self.Is Anchor`))
    (set `self.TotalForce` (0.0 0.0 0.0))
    (for _array_element (`self.Beams`)
      (bind _force (`/Game/Platformer/Bridge/BP_Beam.GetForceAtConnector` _array_element self))
      (set `self.TotalForce` (+ _force (`self.TotalForce`))))
    (`PrimitiveComponent.AddForce` (`self.Sphere`) (`self.TotalForce`) "None" false)))

(fn `UserConstructionScript`
  (bind _sphere (`self.Sphere`))
  (bind _returnvalue (not (`self.Is Anchor`)))
  (`PrimitiveComponent.SetMaterial` (`self.Sphere`) 0 (select `bool` (`self.Is Anchor`) :`false` "/Game/Platformer/Bridge/M_Connector.M_Connector" :`true` "/Game/Platformer/Bridge/MI_Anchor.MI_Anchor" :!type "MaterialInterface Object Reference"))
  (if _returnvalue
    (`|ExecutionSequence`
      (:`then_0`
        (`PrimitiveComponent.SetSimulatePhysics` _sphere _returnvalue))
      (:`then_1`
        (`PrimitiveComponent.SetEnableGravity` _sphere _returnvalue)))))