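; BP_Rotator is a platformer mechanic: a physics-constrained cube whose turning is limited to a set range.
; Each tick it adds the cube's frame-to-frame yaw delta to RotationDone, tracking cumulative rotation, and displays the total on a text render.
; The constraint's Swing1 is free while that total is strictly between zero and Limits, and locked at zero angle otherwise.
; GetPercentage exposes progress as RotationDone divided by Limits.
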(event `self.ReceiveBeginPlay`
  (set `self.PreviousRotation_0` (`SceneComponent.K2_GetComponentRotation` (`self.Cube`))))

(event `self.ReceiveTick`
  (params (DeltaSeconds :type "Float (single-precision)"))
  (bind _rotationdone (`self.RotationDone`))
  (bind _physicsconstraint (`self.PhysicsConstraint`))
  (bind _returnvalue (`SceneComponent.K2_GetComponentRotation` (`self.Cube`)))
  (bind (_returnvalue_roll _returnvalue_pitch _returnvalue_yaw) (`KismetMathLibrary.BreakRotator` (`KismetMathLibrary.NormalizedDeltaRotator` _returnvalue (`self.PreviousRotation_0`))))
  (`TextRenderComponent.K2_SetText` (`self.TextRender`) (`KismetTextLibrary.Conv_DoubleToText` (`self.RotationDone`) "HalfToEven"))
  (set `self.RotationDone` (+ (`self.RotationDone`) _returnvalue_yaw))
  (set `self.PreviousRotation_0` _returnvalue)
  (if (<= _rotationdone 0.0)
    (`PhysicsConstraintComponent.SetAngularSwing1Limit` _physicsconstraint "ACM_Limited" 0.0)
    (elif (>= _rotationdone (`self.Limits`))
      (`PhysicsConstraintComponent.SetAngularSwing1Limit` _physicsconstraint "ACM_Limited" 0.0)
      (else
        (`PhysicsConstraintComponent.SetAngularSwing1Limit` _physicsconstraint "ACM_Free" 0.0)))))

(fn `GetPercentage`
  (returns (Percentage :type "Float (double-precision)"))
  (return (/ (`self.RotationDone`) (`self.Limits`))))

(fn `UserConstructionScript`)