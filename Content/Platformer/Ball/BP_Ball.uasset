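; BP_Ball is a platformer ball actor whose physics can be recorded and rewound.
; On BeginPlay it stores BPBallMovement as its movement component and hands BallMesh to both that component and PPhysicsRecorder.
; Hardcoded key events switch the recorder's state, with A starting a rewind and E resuming recording.
; Movement and rewind logic are delegated to those components, leaving the Blueprint as thin wiring.
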(event `self.ReceiveBeginPlay`
  (bind _output_get (set `self.MovementComponent` (`self.BP_BallMovement`)))
  (`PBallMovementComponent.Initialize` _output_get (`self.BallMesh`))
  (`PPhysicsRecorder.Setup` (`self.PPhysicsRecorder`) (`self.BallMesh`)))

(event `Key|A`
  (params (Key :type "Key Structure"))
  (:`Pressed`
    (set `PPhysicsRecorder.RecordState` "ERS_Rewinding" (`self.PPhysicsRecorder`))))

(event `Key|E`
  (params (Key :type "Key Structure"))
  (:`Pressed`
    (set `PPhysicsRecorder.RecordState` "ERS_Recording" (`self.PPhysicsRecorder`))))

(fn `UserConstructionScript`)